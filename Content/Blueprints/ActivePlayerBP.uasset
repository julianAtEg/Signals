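; ActivePlayerBP is a sprite actor that, going by its name, serves as a spinning marker for the active player.
; Each tick it advances a wrapped Spin angle at a constant rate and sets it as the PaperSprite's relative yaw.
; A SetVisible function shows or hides the sprite and propagates the change to its children.
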(event `self.ReceiveTick`
  (params (DeltaSeconds :type "Float (single-precision)"))
  (bind _output_get (set `self.spin` (mod (+ (`self.spin`) (* DeltaSeconds 45.0)) 360.0)))
  (`SceneComponent.K2_SetRelativeRotation` (`self.PaperSprite`) (`KismetMathLibrary.MakeRotator` 0.0 0.0 _output_get) false false))

(fn `SetVisible`
  (params (visible :type Boolean))
  (`SceneComponent.SetVisibility` (`self.PaperSprite`) visible true))

(fn `UserConstructionScript`)