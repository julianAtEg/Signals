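; Battle mode Blueprint that handles turn-based combat presentation: markers, UI refresh, menu input, animation and floating notifications.
; It finds the active player and target marker actors at start, places them above characters, and shows the active marker only on human turns.
; Menu inputs and UI refreshes go out through dispatchers, with input gated by CanSelectCommands.
; Animations and sounds are handed to SignalsAnimInstance, and floating text widgets spawn at projected screen positions.
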(event `self.ReceiveBeginPlay`
  ;[1 1 1] Initialization
  (bind _outactors (`GameplayStatics.GetAllActorsOfClass` "/Game/Blueprints/ActivePlayerBP.ActivePlayerBP_C"))
  (set `self.ActivePlayerMarker` (`KismetArrayLibrary.Array_Get` _outactors))
  (bind _outactors_2 (`GameplayStatics.GetAllActorsOfClass` "/Game/Blueprints/TargetSpriteBP.TargetSpriteBP_C"))
  (set `self.TargetMarker` (`KismetArrayLibrary.Array_Get` _outactors_2)))

(event `self.OnTurnBeginning`
  (params (character :type "Character Object Reference") (isHuman :type Boolean))
  ;[1 1 1] Active Player Marker
  (`/Game/Blueprints/ActivePlayerBP.SetVisible` (`self.ActivePlayerMarker`) isHuman)
  (if isHuman
    (`self.K2_SetActorLocation` (`self.ActivePlayerMarker`) (+ (`SceneComponent.K2_GetComponentLocation` (`Character.CapsuleComponent` character)) (0.0 0.0 150.0)) false false)
    ;[1 1 1] UI Refresh
    (`self.UpdateControlUIDispatcher` :!label _label)
    (`self.UpdateInfoDispatcher`)))

(event `self.UpdateUI`
  ;[1 1 1] UI Refresh
  (goto _label))

(event `self.HideActiveMarker`
  ;[1 1 1] Active Player Marker
  (`/Game/Blueprints/ActivePlayerBP.SetVisible` (`self.ActivePlayerMarker`) false))

(event `self.ShowActiveMarker`
  ;[1 1 1] Active Player Marker
  (`/Game/Blueprints/ActivePlayerBP.SetVisible` (`self.ActivePlayerMarker`) true))

(event `self.OnMenuLeft`
  ;[1 1 1] Input dispatch
  (if (`self.CanSelectCommands`)
    (`self.MenuEventDispatcher` "MenuLeft")))

(event `self.PlayAnimation`
  (params (character :type "Character Object Reference") (animation :type "String (by ref)") (sound :type "SoundWave Object Reference"))
  ;[1 1 1] Animation Control
  (bind _assignals_anim_instance (cast `SignalsAnimInstance` (`SkeletalMeshComponent.GetAnimInstance` (`Character.Mesh` character))))
  (set `SignalsAnimInstance.NextAnimation` animation _assignals_anim_instance)
  (set `SignalsAnimInstance.Audio` sound _assignals_anim_instance))

(event `self.OnMenuRight`
  ;[1 1 1] Input dispatch
  (if (`self.CanSelectCommands`)
    (`self.MenuEventDispatcher` "MenuRight")))

(event `self.OnMenuSelect`
  ;[1 1 1] Input dispatch
  (if (`self.CanSelectCommands`)
    (`self.MenuEventDispatcher` "MenuSelect")))

(event `self.ShowTargetMarker`
  (params (target :type "Character Object Reference"))
  ;[1 1 1] Target marker
  (`self.K2_SetActorLocation` (`self.TargetMarker`) (+ (`SceneComponent.K2_GetComponentLocation` (`Character.CapsuleComponent` target)) (0.0 0.0 150.0)) false false)
  (`/Game/Blueprints/TargetSpriteBP.SetVisible` (`self.TargetMarker`) true))

(event `self.ReceiveTick`
  (params (DeltaSeconds :type "Float (single-precision)")))

(event `self.HideTargetMarker`
  ;[1 1 1] Target marker
  (`/Game/Blueprints/TargetSpriteBP.SetVisible` (`self.TargetMarker`) false))

(event `self.AddFloatingNotification`
  (params (who :type "Character Object Reference") (text :type "String (by ref)") (color :type "Vector Structure"))
  (bind _returnvalue (`GameplayStatics.GetPlayerController` 0))
  ;[1 1 1] Floating Notifications
  (bind _returnvalue_2 (`|CreateWidget` "/Game/Blueprints/UMGFloatingTextBP.UMGFloatingTextBP_C" _returnvalue))
  (`UserWidget.AddToViewport` _returnvalue_2 0)
  (`/Game/Blueprints/UMGFloatingTextBP.SetScreenPosition` _returnvalue_2 (`PlayerController.ProjectWorldLocationToScreen` _returnvalue (+ (`self.K2_GetActorLocation` who) (0.0 0.0 150.0)))))

(fn `UserConstructionScript`)